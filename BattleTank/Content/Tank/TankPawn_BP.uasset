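; Player tank pawn Blueprint that wires components and input for driving, aiming and firing.
; On BeginPlay it passes the barrel and turret to the TankAiming component and both tracks to TankMovement.
; Fire and move inputs forward to those components.
; Aim axes rotate the camera rig, with yaw on an azimuth gimbal and pitch on the spring arm, each scaled by a sensitivity multiplier.
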(event `self.ReceiveBeginPlay`
  (`TankAimingComponent.InitialiseAiming` (`self.TankAiming`) (`self.TankBarrel`) (`self.TankTurret`))
  (`TankMovementComponent.InitialiseMovement` (`self.TankMovement`) (`self.LeftTrack`) (`self.RightTrack`)))

(event `InputAction|Fire`
  (params (Key :type "Key Structure"))
  ;[1 1 1] Fire Input (Mouse Left)
  (:`Pressed`
    (`TankAimingComponent.Fire` (`self.TankAiming`))))

(event `InputAxis|Aim Azimuth`
  (params (AxisValue :type "Float (single-precision)"))
  ;[1 1 1] Camera Movement (Pitch & Yaw)
  (`SceneComponent.K2_AddLocalRotation` (`self.AzimuthGimbal`) (`KismetMathLibrary.MakeRotator` 0.0 0.0 (* AxisValue (`self.XSensitivityMult`))) false false))

(event `InputAxis|Move Forward`
  (params (AxisValue :type "Float (single-precision)"))
  ;[1 1 1] Tank Movement Setup
  (`TankMovementComponent.IntendMoveForward` (`self.TankMovement`) AxisValue))

(event `InputAxis|Aim Elevation`
  (params (AxisValue :type "Float (single-precision)"))
  ;[1 1 1] Camera Movement (Pitch & Yaw)
  (`SceneComponent.K2_AddLocalRotation` (`self.SpringArm`) (`KismetMathLibrary.MakeRotator` 0.0 (* AxisValue (`self.YSensitivityMult`))) false false))

(event `InputAxis|Move Sideways`
  (params (AxisValue :type "Float (single-precision)"))
  ;[1 1 1] Tank Movement Setup
  (`TankMovementComponent.IntendMoveSideways` (`self.TankMovement`) AxisValue))

(fn `UserConstructionScript`)