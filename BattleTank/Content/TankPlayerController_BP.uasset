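; Tank player controller Blueprint that creates the player HUD and handles the pause menu.
; When the aiming component and tank are found, it spawns the PlayerUI widget and passes it both references.
; BeginPlay creates a hidden pause menu and stores the viewport center.
; The Pause input toggles the menu, game pause, input mode and cursor visibility, then moves the mouse to that center.
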(event `self.FoundAimingComponentAndTank`
  (params (AimingCompRef :type "TankAimingComponent Object Reference") (TankReference :type "Tank Object Reference"))
  (bind _returnvalue (`|CreateWidget` "/Game/UI/PlayerUI.PlayerUI_C"))
  (`UserWidget.AddToViewport` _returnvalue 0)
  (set `/Game/UI/PlayerUI.BPAimingCompRef` AimingCompRef _returnvalue)
  (set `/Game/UI/PlayerUI.TankReference` TankReference _returnvalue))

(event `self.ReceiveBeginPlay`
  (bind (_sizex _sizey) (`self.GetViewportSize`))
  (bind _pausemenuvar (`self.PauseMenuVar`))
  (bind _returnvalue (`|CreateWidget` "/Game/UI/PauseMenu.PauseMenu_C"))
  (set `self.PauseMenuVar` _returnvalue)
  (set `/Game/UI/PauseMenu.PlayerControllerReference` self _pausemenuvar)
  (`Widget.SetVisibility` _pausemenuvar "Hidden")
  (`UserWidget.AddToViewport` _pausemenuvar 0)
  (set `self.PosX` (/ _sizex 2))
  (set `self.PosY` (/ _sizey 2)))

(event `InputAction|Pause` :paused true
  (params (Key :type "Key Structure"))
  (:`Pressed`
    (`self.ToggleVisibility`)))

(fn `ToggleVisibility`
  (bind _pausemenuvar (`self.PauseMenuVar`))
  (if (`self.IsVisible`)
    (`Widget.SetVisibility` _pausemenuvar "Hidden")
    (`WidgetBlueprintLibrary.SetInputMode_GameOnly` self)
    (bind _output_get (set `self.IsVisible` false))
    (`GameplayStatics.SetGamePaused` _output_get)
    (set `self.bShowMouseCursor` false)
    (else
      (`Widget.SetVisibility` _pausemenuvar "Visible")
      (`WidgetBlueprintLibrary.SetInputMode_GameAndUIEx` self _pausemenuvar "LockAlways")
      (bind _output_get_2 (set `self.IsVisible` true))
      (`GameplayStatics.SetGamePaused` _output_get_2)
      (set `self.bShowMouseCursor` true)))
  (`self.SetMouseLocation` (`self.PosX`) (`self.PosY`))
  (return))

(fn `UserConstructionScript`)